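; Backup hospital dialogue trigger Blueprint that feeds dialogue rows to a HUD widget and has a camera slide.
; Disconnected setup logic would load Hosp_Dialogue_2a into a struct array, create WBP_HospitalDialogueBox and call DialogueRun.
; DialogueRun updates the box with the current row unless it is marked EndScene.
; LerpCam moves the camera between two spline points by timeline; its speaker branches and SlideCamera are empty.
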(event `self.ReceiveBeginPlay`)

(event `DialogueRun`
  (bind _output (`|GetArrayItem` (`self.HospitalDialogueArray`) (`self.DialogueRow`)))
  ;[1 1 1] Starts dialogue
  (if (not (`KismetStringLibrary.EqualEqual_StrStr` (`.EndScene_11_373555584251DA7F57404CA2160EFDEE` (break `/Game/Louis_Blueprints/S_HospitalDialogue` _output)) "Yes"))
    (`/Game/Louis_Blueprints/WBP_HospitalDialogueBox.UpdateDialogueBox` (`self.HospitalDialogueHUD Ref`) _output)
    (`KismetSystemLibrary.PrintString` "1")))

(event `LerpCam`
  (bind _spline (`self.Spline`))
  (switch `/Game/Louis_Blueprints/Enum_HospitalDialogueSpeaker` (`self.SpeakerEnum`)
    (:`NewEnumerator0`
      (bind (_direction _cammove) (`Timeline|Lerp To Charlie` :!label _label)
        (:`Update`
          (`SceneComponent.K2_SetWorldLocation` (`self.Camera`) (`KismetMathLibrary.VLerp` (`SplineComponent.GetLocationAtSplinePoint` _spline 0 "World") (`SplineComponent.GetLocationAtSplinePoint` _spline 1 "World") _cammove) false false))))
    (:`NewEnumerator1`
      (goto _label))))

(fn `SlideCamera`
  (params (SpeakerEnum :type "/Game/Louis_Blueprints/Enum_HospitalDialogueSpeaker Enum" :default "NewEnumerator0")))

(fn `UserConstructionScript`)