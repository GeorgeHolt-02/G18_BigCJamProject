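; BP_TempShooter is a temporary shooter pawn that player controller 0 possesses on BeginPlay.
; Clamped mouse Y input accumulates into a 0–1 value that lerps the Sphere linearly between the spline's first two points.
; Left click spawns a BP_TempBullet at the Sphere facing world +X, with a DoOnce reset on release to allow one shot per press.
; Debug "Hello" prints remain on possession and firing.
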(event `self.ReceiveBeginPlay`
  (`Controller.Possess` (`GameplayStatics.GetPlayerController` 0) self)
  (`KismetSystemLibrary.PrintString` "Hello"))

(event `InputAxis|MouseYAxis`
  (params (AxisValue :type "Float (single-precision)"))
  (bind _spline (`self.Spline`))
  (bind _output_get (set `self.MouseYPos` (`KismetMathLibrary.FClamp` (+ (`KismetMathLibrary.FClamp` AxisValue -0.02 0.02) (`self.MouseYPos`)))))
  (`SceneComponent.K2_SetWorldLocation` (`self.Sphere`) (`KismetMathLibrary.VLerp` (`SplineComponent.GetLocationAtSplinePoint` _spline 0 "World") (`SplineComponent.GetLocationAtSplinePoint` _spline 1 "World") _output_get) false false))

(event `InputAction|LeftClick`
  (params (Key :type "Key Structure"))
  (bind _returnvalue (`SceneComponent.K2_GetComponentLocation` (`self.Sphere`)))
  (:`Pressed`
    (`KismetSystemLibrary.PrintString` "Hello")
    (`/Engine/EditorBlueprintResources/StandardMacros.DoOnce` false :!label _label
      (:`Completed`
        (`KismetSystemLibrary.PrintString` "Hello")
        (`|SpawnActorFromClass` "/Game/Louis_Blueprints/BP_TempBullet.BP_TempBullet_C" (`KismetMathLibrary.MakeTransform` _returnvalue (`KismetMathLibrary.FindLookAtRotation` _returnvalue (+ _returnvalue (10.0 0.0 0.0)))) "Undefined" "OverrideRootScale" null null))))
  (:`Released`
    (goto _label :!via `Reset`)))

(fn `UserConstructionScript`)