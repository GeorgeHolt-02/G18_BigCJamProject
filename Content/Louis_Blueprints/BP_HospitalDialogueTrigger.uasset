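; Hospital dialogue trigger that starts a conversation at BeginPlay and provides a sliding camera for its speakers.
; BeginPlay copies the Hosp_Dialogue_2a data table into a struct array, then passes it and itself to an on-screen dialogue widget.
; DialogueRun sends the current row to that widget unless it is flagged EndScene.
; LerpCam uses a timeline to move the camera between two spline points for Charlie, reversing it for Nurse.
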(event `self.ReceiveBeginPlay`
  (bind _hospitaldialoguehud_ref (`self.HospitalDialogueHUD Ref`))
  (`|ExecutionSequence`
    (:`then_0`
      (`Controller.Possess` (`GameplayStatics.GetPlayerController` 0) null))
    (:`then_1`
      ;[1 1 1] Converts Data table into struct array for processing
      (bind _outrownames (`DataTableFunctionLibrary.GetDataTableRowNames` "/Game/Louis_Blueprints/Hosp_Dialogue_2a.Hosp_Dialogue_2a"))
      (for _array_element _outrownames
        (bind _returnvalue (`|GetDataTableRow` "/Game/Louis_Blueprints/Hosp_Dialogue_2a.Hosp_Dialogue_2a" _array_element)
          (:`then`
            (`KismetArrayLibrary.Array_Add` (`self.HospitalDialogueArray`) _returnvalue)))))
    (:`then_2`
      ;[1 1 1] Spawns widget and adds it to viewport, assigns created array to it for it to work with
      (bind _returnvalue_2 (`|CreateWidget` "/Game/Louis_Blueprints/WBP_HospitalDialogueBox.WBP_HospitalDialogueBox_C"))
      (bind _output_get (set `self.HospitalDialogueHUD Ref` _returnvalue_2))
      (set `/Game/Louis_Blueprints/WBP_HospitalDialogueBox.DialogueStructArray` (`self.HospitalDialogueArray`) _hospitaldialoguehud_ref)
      (set `/Game/Louis_Blueprints/WBP_HospitalDialogueBox.TriggerActor` self _hospitaldialoguehud_ref)
      (`UserWidget.AddToViewport` _output_get 0)
      (`self.DialogueRun`))))

(event `DialogueRun`
  (bind _output (`|GetArrayItem` (`self.HospitalDialogueArray`) (`self.DialogueRow`)))
  ;[1 1 1] Starts dialogue
  (if (not (`KismetStringLibrary.EqualEqual_StrStr` (`.EndScene_11_373555584251DA7F57404CA2160EFDEE` (break `/Game/Louis_Blueprints/S_HospitalDialogue` _output)) "Yes"))
    (`/Game/Louis_Blueprints/WBP_HospitalDialogueBox.UpdateDialogueBox` (`self.HospitalDialogueHUD Ref`) _output)
    (`KismetSystemLibrary.PrintString` "1")))

(event `LerpCam`
  (bind _spline (`self.Spline`))
  (switch `/Game/Louis_Blueprints/Enum_HospitalDialogueSpeaker` (`self.SpeakerEnum`)
    (:`NewEnumerator0`
      (bind (_direction _cammove) (`Timeline|Lerp To Charlie` :!label _label)
        (:`Update`
          (`SceneComponent.K2_SetWorldLocation` (`self.Camera`) (`KismetMathLibrary.VLerp` (`SplineComponent.GetLocationAtSplinePoint` _spline 1 "World") (`SplineComponent.GetLocationAtSplinePoint` _spline 0 "World") _cammove) false false))))
    (:`NewEnumerator1`
      (goto _label :!via `Reverse`))))

(fn `SlideCamera`
  (params (SpeakerEnum :type "/Game/Louis_Blueprints/Enum_HospitalDialogueSpeaker Enum" :default "NewEnumerator0")))

(fn `UserConstructionScript`)