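; Enemy spawn volume that spawns waves of temporary enemies along splines, followed by a boss.
; BeginPlay spawns the first wave and starts a five-second timer, optionally looping, that advances the wave index.
; Each WaveIndexArray entry selects one of three splines and an enemy count, with SubdivideSpline computing evenly spaced world locations.
; When the index equals the array length, the boss spawns at the first previously computed location.
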(event `self.ReceiveBeginPlay`
  (`self.Spawn Event`)
  (`KismetSystemLibrary.K2_SetTimerDelegate` (delegate `Spawn Event`) 5.0 (`self.LoopSpawn`)))

(event `Spawn Event`
  (bind _waveindex (`self.WaveIndex`))
  (`self.SpawnEnemies` _waveindex)
  (`/Engine/EditorBlueprintResources/StandardMacros.IncrementInt` _waveindex))

(fn `SpawnEnemies`
  (params (WaveIndex :type Integer))
  (bind _output (`|GetArrayItem` (`self.WaveIndexArray`) WaveIndex))
  (`KismetSystemLibrary.PrintString` (`KismetStringLibrary.Conv_IntToString` WaveIndex))
  (if (== (`KismetArrayLibrary.Array_Length` (`self.WaveIndexArray`)) WaveIndex)
    (`|SpawnActorFromClass` "/Game/Louis_Blueprints/BP_TempBossEnemy.BP_TempBossEnemy_C" (`KismetMathLibrary.MakeTransform` (`|GetArrayItem` (`self.SpawnVecArray`))) "Undefined" "OverrideRootScale" null null)
    (else
      (`KismetSystemLibrary.PrintString` (`KismetStringLibrary.Conv_IntToString` _output))
      (switch `int` _output
        (:`Default`
          (bind _vecarray (`self.SubdivideSpline` 3 (`self.Spline1`) :!label _label))
          (for _array_element _vecarray
            (`|SpawnActorFromClass` "/Game/Louis_Blueprints/BP_TempEnemy.BP_TempEnemy_C" (`KismetMathLibrary.MakeTransform` _array_element) "Undefined" "OverrideRootScale" null null)))
        (:`0`
          (goto _label))
        (:`1`
          (bind _vecarray_2 (`self.SubdivideSpline` 7 (`self.Spline2`)))
          (for _array_element_2 _vecarray_2
            (`|SpawnActorFromClass` "/Game/Louis_Blueprints/BP_TempEnemy.BP_TempEnemy_C" (`KismetMathLibrary.MakeTransform` _array_element_2) "Undefined" "OverrideRootScale" null null)))
        (:`2`
          (bind _vecarray_3 (`self.SubdivideSpline` 5 (`self.Spline3`)))
          (for _array_element_3 _vecarray_3
            (`|SpawnActorFromClass` "/Game/Louis_Blueprints/BP_TempEnemy.BP_TempEnemy_C" (`KismetMathLibrary.MakeTransform` _array_element_3) "Undefined" "OverrideRootScale" null null)))))))

(fn `SubdivideSpline`
  (params (SpawnNumber :type Integer) (Spline :type "SplineComponent Object Reference"))
  (returns (VecArray :type "Array of Vector Structure"))
  (bind _returnvalue (- SpawnNumber 1))
  (`KismetArrayLibrary.Array_Clear` (`self.SpawnVecArray`))
  (set `self.SegmentLength` (/ (`SplineComponent.GetSplineLength` Spline) _returnvalue))
  (for _index (range (+ _returnvalue 1))
    (`KismetArrayLibrary.Array_Add` (`self.SpawnVecArray`) (`SplineComponent.GetLocationAtDistanceAlongSpline` Spline (* _index (`self.SegmentLength`)) "World")))
  (return (`self.SpawnVecArray`)))

(fn `UserConstructionScript`)